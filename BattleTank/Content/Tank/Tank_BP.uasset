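; Player-controllable tank Blueprint that wires input to aiming and movement components and hooks up a healthbar widget.
; On BeginPlay it passes turret and barrel to Aiming, both tracks to Movement, and itself to the Healthbar widget.
; Forward and turn axes feed Movement, and Fire triggers Aiming.
; Aim axes rotate the camera rig's azimuth gimbal and spring arm, scaled by delta time for frame-rate independence.
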(event `self.ReceiveBeginPlay`
  (`TankAimingComponent.Initialize` (`self.Aiming`) (`self.Turret`) (`self.Barrel`))
  (`TankMovementComponent.Initialize` (`self.Movement`) (`self.Left Track`) (`self.Right Track`))
  (`self.InitializeHealthbarWidget`))

(event `InputAxis|AimAzimuth`
  (params (AxisValue :type "Float (single-precision)"))
  ;[1 1 1] Aim Input Binding
  (`SceneComponent.K2_AddLocalRotation` (`self.Azimuth Gimbal`) (`KismetMathLibrary.MakeRotator` 0.0 0.0 (* AxisValue (`GameplayStatics.GetWorldDeltaSeconds`) 100.0)) false false))

(event `InputAxis|MoveForward`
  (params (AxisValue :type "Float (single-precision)"))
  ;[1 1 1] Movement Input Binding
  (`TankMovementComponent.MoveForward` (`self.Movement`) AxisValue))

(event `InputAxis|TurnRight`
  (params (AxisValue :type "Float (single-precision)"))
  ;[1 1 1] Movement Input Binding
  (`TankMovementComponent.TurnRight` (`self.Movement`) AxisValue))

(event `InputAxis|AimElevation`
  (params (AxisValue :type "Float (single-precision)"))
  ;[1 1 1] Aim Input Binding
  (`SceneComponent.K2_AddLocalRotation` (`self.SpringArm`) (`KismetMathLibrary.MakeRotator` 0.0 (* AxisValue (`GameplayStatics.GetWorldDeltaSeconds`) 100.0)) false false))

(event `InputAction|Fire`
  (params (Key :type "Key Structure" :default "AnyKey"))
  ;[1 1 1] Aim Input Binding
  (:`Pressed`
    (`TankAimingComponent.Fire` (`self.Aiming`))))

(fn `InitializeHealthbarWidget`
  (bind _ashealthbar (cast `/Game/UI/Healthbar` (`WidgetComponent.GetUserWidgetObject` (`self.Widget`)))
    (:`then`
      (set `/Game/UI/Healthbar.Tank` self _ashealthbar))
    (:`CastFailed`
      _))
  (return))

(fn `UserConstructionScript`)